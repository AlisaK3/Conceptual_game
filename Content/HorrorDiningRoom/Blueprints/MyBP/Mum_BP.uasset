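; Mum NPC for the horror dining room that runs a scripted conversation, reveals hidden decals as it progresses and triggers the ending screen.
; Player overlap creates the dialog widget and leaving removes it.
; Each Interact passes the MumText lines to the widget and advances its row through a resettable DoOnce, closing it after the last line.
; Specific rows unhide decals, and a late row shows End_Widget after a delay.
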(event Custom|resetDialog
  (bind _dialogui (Variables|Default|GetDialogUI))
  (Utilities|FlowControl|DoOnce false) ; enters at Reset
)

(event Collision|EventActorEndOverlap
  (params (OtherActor :type Actor%20Object%20Reference))
  (Utilities|Casting|CastToFirstPersonCharacter OtherActor)
  (Widget|RemovefromParent (stale Collision|EventActorBeginOverlap _output_get)))

(event Collision|EventActorBeginOverlap
  (params (OtherActor :type Actor%20Object%20Reference))
  (Utilities|Casting|CastToFirstPersonCharacter OtherActor)
  (bind _returnvalue (UserInterface|CreateWidget "/Game/HorrorDiningRoom/Blueprints/MyBP/Dialog_Widget.Dialog_Widget_C"))
  (bind _output_get (Variables|Default|SetDialogUI _returnvalue))
  (UserInterface|Viewport|AddtoViewport _output_get 0))

(event EventInteract
  (bind _dialogui (Variables|Default|GetDialogUI))
  (Utilities|FlowControl|DoOnce false
    (:Completed
      (Variables|/Game/HorrorDiningRoom/Blueprints/MyBP/Dialog_Widget.Dialog_Widget_C|SetText _dialogui (Variables|Default|GetMumText))
      (Widget|SetVisibility (Variables|/Game/HorrorDiningRoom/Blueprints/MyBP/Dialog_Widget.Dialog_Widget_C|GetTextBlock_281 _dialogui) "Visible")
      (if (> (+ (Variables|/Game/HorrorDiningRoom/Blueprints/MyBP/Dialog_Widget.Dialog_Widget_C|Gettextrow (Variables|Default|GetDialogUI)) 1) (- (Utilities|Array|Length (Variables|Default|GetMumText)) 1))
        (Widget|RemovefromParent (Variables|Default|GetDialogUI))
        (CallFunction|ResetDialog)
        (else
          (bind _output_get (Variables|/Game/HorrorDiningRoom/Blueprints/MyBP/Dialog_Widget.Dialog_Widget_C|Settextrow (Variables|Default|GetDialogUI) (+ (Variables|/Game/HorrorDiningRoom/Blueprints/MyBP/Dialog_Widget.Dialog_Widget_C|Gettextrow (Variables|Default|GetDialogUI)) 1)))
          (bind _output_get_2 (Variables|Default|Setcurrentrow _output_get))
          (CallFunction|ResetDialog)
          (if (== _output_get_2 7)
            (Rendering|SetVisibility (Variables|Default|GetDecal) true false)
            (elif (== _output_get_2 13)
              (Rendering|SetVisibility (Variables|Default|GetDecal2) true false)
              (elif (== _output_get_2 21)
                (Rendering|SetVisibility (Variables|Default|GetDecal4) true false)
                (elif (== _output_get_2 23)
                  (Utilities|FlowControl|Delay 1e+01)
                  (bind _returnvalue (UserInterface|CreateWidget "/Game/HorrorDiningRoom/Blueprints/MyBP/End_Widget.End_Widget_C"))
                  (UserInterface|Viewport|AddtoViewport _returnvalue 0))))))))))

(event EventBeginPlay
  (Rendering|SetVisibility (Variables|Default|GetDecal) false false))

(fn ConstructionScript)